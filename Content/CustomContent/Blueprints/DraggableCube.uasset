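; Draggable cube actor that the 2D character grabs via OnInteract and drags for as long as E is held.
; Interacting stores the cube's offset from the player capsule, which Tick reapplies by teleport-free, non-swept moves while ignoring Pawn collision.
; A short debug-drawn trace along the player's forward vector halts movement and restores Pawn blocking on a hit.
; Releasing E restores blocking and clears the character's IsDragging flag.
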(event EventOnInteract
  ;[1 1 1] Dragging
  (CallFunction|SetwhenInteract))

(event EventTick
  (params (DeltaSeconds :type Float%20%28single-precision%29))
  ;[1 1 1] Dragging
  (if (Game|Player|IsInputKeyDown (Game|GetPlayerController 0) "E")
    (Variables|Default|SetisEKeyPressed true)
    (if (Variables|Default|GethasInteract)
      (bind _willcollide (CallFunction|CheckCollisions))
      (if _willcollide
        (CallFunction|EnablePawnCollision true)
        (else
          (CallFunction|EnablePawnCollision false)
          (Transformation|SetWorldLocation (Variables|Default|GetCube) (+ (Transformation|GetWorldLocation (Variables|/Script/Engine.Character|GetCapsuleComponent (Game|GetPlayerCharacter 0))) (Variables|Default|GetdraggingVector)) false false))))
    (else
      (CallFunction|SetwhenKeyReleased))))

(fn ConstructionScript)

(fn GetPlayerForwardDirection
  (if (>= (.X (Math|Vector|BreakVector (Transformation|GetActorForwardVector (Game|Player|GetPlayerPawn 0)))) 0.0)
    (return "NewEnumerator0")
    (else
      (return "NewEnumerator1"))))

(fn GetPlayerRelativeDirection
  (if (>= (.X (Math|Vector|BreakVector (Transformation|GetWorldLocation (Variables|Default|GetCube)))) (.X (Math|Vector|BreakVector (Transformation|GetWorldLocation (Variables|/Script/Engine.Character|GetCapsuleComponent (Game|GetPlayerCharacter 0))))))
    (return "NewEnumerator0")
    (else
      (return "NewEnumerator1"))))

(fn CheckCollisions
  (bind _cube (Variables|Default|GetCube))
  (bind _boxextent (Collision|GetComponentBounds _cube))
  (bind _returnvalue (Transformation|GetWorldLocation _cube))
  (bind _returnvalue_2 (* _boxextent "0.000000,0.000000,0.500000"))
  (bind _returnvalue_3 (+ _returnvalue _returnvalue_2))
  (bind _returnvalue_4 (Collision|LineTraceByChannel _returnvalue_3 (+ _returnvalue_3 (* (Math|Vector|GetForwardVector (Game|GetPlayerCharacter 0)) 75.0)) "TraceTypeQuery1" false 0 "ForOneFrame"))
  (return _returnvalue_4))

(fn SetwhenKeyReleased
  (if (Variables|Default|GetisEKeyPressed)
    (Variables|Default|SetisEKeyPressed false)
    (Variables|Default|SethasInteract false)
    (bind _as2dcharacter (Utilities|Casting|CastTo2DCharacter (Game|Player|GetPlayerPawn 0)))
    (Variables|/Game/2DSideScrollerBP/Blueprints/2DCharacter.2DCharacter_C|SetisDragging _as2dcharacter false)
    (Collision|SetCollisionResponsetoChannel (Variables|Default|GetCube) "ECC_Pawn" "ECR_Block")))

(fn SetwhenInteract
  (Variables|Default|SethasInteract true)
  (Variables|Default|SetdraggingVector (- (Transformation|GetWorldLocation (Variables|Default|GetCube)) (Transformation|GetWorldLocation (Variables|/Script/Engine.Character|GetCapsuleComponent (Game|GetPlayerCharacter 0)))))
  (bind _as2dcharacter (Utilities|Casting|CastTo2DCharacter (Game|Player|GetPlayerPawn 0)))
  (Variables|/Game/2DSideScrollerBP/Blueprints/2DCharacter.2DCharacter_C|SetisDragging _as2dcharacter true))

(fn EnablePawnCollision
  (params (enabled :type Boolean))
  (bind _cube (Variables|Default|GetCube))
  (if enabled
    (Collision|SetCollisionResponsetoChannel _cube "ECC_Pawn" "ECR_Block")
    (else
      (Collision|SetCollisionResponsetoChannel _cube "ECC_Pawn" "ECR_Ignore"))))