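; PressureCube is a pressure-plate style cube that squashes vertically while something overlaps its collision box.
; Begin and end overlap events set an IsOverlapped flag, which Tick uses to raise or lower a clamped alpha over about a quarter second.
; That alpha lerps the root component's Z scale between resting and pressed heights, leaving X and Y unchanged.
; It only animates; it triggers nothing else.
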(event OnComponentEndOverlap(CollisionBox)
  (params (OtherActor :type Actor%20Object%20Reference) (OtherComp :type Primitive%20Component%20Object%20Reference) (OtherBodyIndex :type Integer))
  (Variables|Default|SetisOverlapped false))

(event OnComponentBeginOverlap(CollisionBox)
  (params (OtherActor :type Actor%20Object%20Reference) (OtherComp :type Primitive%20Component%20Object%20Reference) (OtherBodyIndex :type Integer) (bFromSweep :type Boolean) (SweepResult :type Hit%20Result%20Structure%20%28by%20ref%29))
  (Variables|Default|SetisOverlapped true))

(event EventTick
  (params (DeltaSeconds :type Float%20%28single-precision%29))
  (CallFunction|AddDeltaTimetoAlpha DeltaSeconds)
  (CallFunction|ScalewithOverlappingAlpha))

(fn ConstructionScript)

(fn ScalewithOverlappingAlpha
  (bind _defaultsceneroot (Variables|Default|GetDefaultSceneRoot))
  (bind _returnvalue (Transformation|GetRelativeTransform _defaultsceneroot))
  (bind _scale (Math|Transform|BreakTransform _returnvalue))
  (bind (_x _y) (Math|Vector|BreakVector _scale))
  (Transformation|SetRelativeScale3D (Variables|Default|GetDefaultSceneRoot) (Math|Vector|MakeVector _x _y (Math|Float|Lerp 0.5 0.35 (Variables|Default|GetoverlappingAlpha)))))

(fn AddDeltaTimetoAlpha
  (params (deltaTime :type Float%20%28single-precision%29))
  (LocalVariables|SetScaledDeltaTime (* deltaTime 4.0))
  (if (Variables|Default|GetisOverlapped)
    (Variables|Default|SetoverlappingAlpha (Math|Float|Clamp(Float) (+ (Variables|Default|GetoverlappingAlpha) (LocalVariables|GetScaledDeltaTime))))
    (else
      (Variables|Default|SetoverlappingAlpha (Math|Float|Clamp(Float) (- (Variables|Default|GetoverlappingAlpha) (LocalVariables|GetScaledDeltaTime)))))))