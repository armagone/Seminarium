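; Pressure plate door that raises Door while something overlaps PressureCollisionBox and lowers it once the overlaps end.
; An overlap counter sets IsOverlapped, which Tick uses to ramp a clamped OverlappingAlpha up or down over a fraction of a second.
; Door moves in world Z by the per-frame change in alpha, so it needs no stored start position.
; ScaleWithOverlappingAlpha would squash PressureBox with the alpha, but nothing here calls it.
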(event OnComponentEndOverlap(PressureCollisionBox)
  (params (OtherActor :type Actor%20Object%20Reference) (OtherComp :type Primitive%20Component%20Object%20Reference) (OtherBodyIndex :type Integer))
  (bind _result (Math|Integer|DecrementInt (Variables|Default|GetoverlapCounter))
    (:%20%20
      (if (not (> _result 0))
        (Variables|Default|SetisOverlapped false)))))

(event OnComponentBeginOverlap(PressureCollisionBox)
  (params (OtherActor :type Actor%20Object%20Reference) (OtherComp :type Primitive%20Component%20Object%20Reference) (OtherBodyIndex :type Integer) (bFromSweep :type Boolean) (SweepResult :type Hit%20Result%20Structure%20%28by%20ref%29))
  (Math|Integer|IncrementInt (Variables|Default|GetoverlapCounter)
    (:%20%20
      (Variables|Default|SetisOverlapped true))))

(event EventTick
  (params (DeltaSeconds :type Float%20%28single-precision%29))
  (CallFunction|AddDeltaTimetoAlpha DeltaSeconds)
  (CallFunction|MoveDoorwithAlpha)
  (Variables|Default|SetlastOverlappingAlpha (Variables|Default|GetoverlappingAlpha)))

(fn ConstructionScript)

(fn ScalewithOverlappingAlpha
  (bind _pressurebox (Variables|Default|GetPressureBox))
  (bind _returnvalue (Transformation|GetRelativeTransform _pressurebox))
  (bind _scale (Math|Transform|BreakTransform _returnvalue))
  (bind (_x _y) (Math|Vector|BreakVector _scale))
  (Transformation|SetRelativeScale3D (Variables|Default|GetPressureBox) (Math|Vector|MakeVector _x _y (Math|Float|Lerp 0.7 0.35 (Variables|Default|GetoverlappingAlpha)))))

(fn AddDeltaTimetoAlpha
  (params (deltaTime :type Float%20%28single-precision%29))
  (LocalVariables|SetScaledDeltaTime (* deltaTime 4.0))
  (if (Variables|Default|GetisOverlapped)
    (Variables|Default|SetoverlappingAlpha (Math|Float|Clamp(Float) (+ (Variables|Default|GetoverlappingAlpha) (LocalVariables|GetScaledDeltaTime))))
    (else
      (Variables|Default|SetoverlappingAlpha (Math|Float|Clamp(Float) (- (Variables|Default|GetoverlappingAlpha) (LocalVariables|GetScaledDeltaTime)))))))

(fn MoveDoorwithAlpha
  (bind _door (Variables|Default|GetDoor))
  (bind _returnvalue (Transformation|GetWorldLocation _door))
  (bind (_x _y _z) (Math|Vector|BreakVector _returnvalue))
  (Transformation|SetWorldLocation (Variables|Default|GetDoor) (Math|Vector|MakeVector _x _y (+ (* (- (Variables|Default|GetoverlappingAlpha) (Variables|Default|GetlastOverlappingAlpha)) 6e+02) _z)) false false))